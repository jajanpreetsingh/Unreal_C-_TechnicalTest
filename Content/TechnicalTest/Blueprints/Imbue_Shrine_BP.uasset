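; Imbue shrine that alters the element of pickables dropped on its magnet by Set, Add, Remove or Split, or creates spheres by Merge.
; Construction script shows each mode's sign meshes; BeginPlay colors the base from the game mode's elemental definition.
; Split spreads an element across linked pedestals, retrying on Tick until all are free.
; Merge polls for occupied pedestals, spawning the combined sphere and updating or destroying sources, with optional element filtering for both.
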(event `self.ReceiveBeginPlay`
  (`self.RefreshMaterial`))

(event `self.PickableMagnet.OnDropEvent`
  (params (pickable :type "PickableComponent Object Reference"))
  (bind _returnvalue (`self.GetComponentByClass` (`ActorComponent.GetOwner` pickable) "/Script/TechnicalTest.ElementalComponent"))
  (bind _elementtype (`ElementalComponent.ElementType` (`self.Elemental`)))
  (switch `/Game/TechnicalTest/Enum/ElementImbueType` (`self.ImbueType`)
    (:`NewEnumerator0`
      (`ElementalComponent.SetElement` _returnvalue _elementtype))
    (:`NewEnumerator1`
      (`ElementalComponent.AddElements` _returnvalue _elementtype))
    (:`NewEnumerator2`
      (`ElementalComponent.RemoveElements` _returnvalue _elementtype))
    (:`NewEnumerator3`
      (`self.SplitElement` _returnvalue))))

(event `self.ReceiveTick`
  (params (DeltaSeconds :type "Float (single-precision)"))
  (`|ExecutionSequence`
    (:`then_0`
      ;[1 1 1] Split
      (if (`self.bWaitingForSplit`)
        (`self.SplitElement` (`self.GetComponentByClass` (`ActorComponent.GetOwner` (`PickableMagnetComponent.CurrentPickable` (`self.PickableMagnet`))) "/Script/TechnicalTest.ElementalComponent"))))
    (:`then_1`
      ;[1 1 1] Merge
      (if (`|EnumEquality` (`self.ImbueType`) "NewEnumerator4")
        (`self.TryMerge`)))))

(fn `RefreshMaterial`
  (bind _asttgame_mode_bp (cast `/Game/TechnicalTest/Blueprints/TTGameMode_BP` (`GameplayStatics.GetGameMode`)))
  (bind _returnvalue (`TTGameMode.GetElementalDefinition` _asttgame_mode_bp (`ElementalComponent.ElementType` (`self.Elemental`))))
  (`PrimitiveComponent.SetMaterial` (`self.Base`) 0 (`.Material` (break `ElementalDefinition` _returnvalue))))

(fn `SplitElement`
  (params (ElementalToSplit :type "ElementalComponent Object Reference"))
  (locals (bValid :type Boolean :default true))
  (bind _splitormergevalidstate (`self.SplitOrMergeValidState`))
  (bind _currentpickable (`PickableMagnetComponent.CurrentPickable` (`self.PickableMagnet`)))
  (set `self.bWaitingForSplit` false)
  (`/Engine/EditorBlueprintResources/StandardMacros.IsValid` (`PickableMagnetComponent.CurrentPickable` (`self.PickableMagnet`))
    (:`Is Valid`
      (bind _output_get (set `local.bValid` (and (or (`KismetArrayLibrary.Array_Contains` _splitormergevalidstate (`ElementalComponent.ElementType` ElementalToSplit)) (== (`KismetArrayLibrary.Array_Length` _splitormergevalidstate) 0)) (`ElementalComponent.IsSplittable` ElementalToSplit))))
      (if _output_get
        (for _array_element (`self.LinkedPedestral`)
          ;[1 1 1] All Pedestral are free
          (set `local.bValid` (and (`PickableMagnetComponent.IsAvailable` (`/Game/TechnicalTest/Blueprints/Pedestral_BP.PickableMagnet` _array_element)) (`local.bValid`))))
        (if (`local.bValid`)
          (bind _returnvalue (`ElementalComponent.SplitElement` ElementalToSplit (`KismetArrayLibrary.Array_Length` (`self.LinkedPedestral`))))
          (`self.K2_DestroyActor` (`ActorComponent.GetOwner` _currentpickable))
          (`PickableMagnetComponent.DetachPickable` (`self.PickableMagnet`) _currentpickable)
          (for (_array_element_2 _array_index) (`self.LinkedPedestral`)
            (bind _output (`|GetArrayItem` _returnvalue _array_index))
            ;[1 1 1] Never spawn a null element
            (if (!= _output 0)
              (`/Game/TechnicalTest/Blueprints/Pedestral_BP.SpawnElementalSphere` _array_element_2 _output)))
          (else
            (set `self.bWaitingForSplit` true)))))))

(fn `TryMerge`
  (locals (bValid :type Boolean :default true) (Elements :type "Array of ElementalComponent Object Reference"))
  (bind _splitormergevalidstate (`self.SplitOrMergeValidState`))
  (bind (_returnvalue_location _returnvalue_rotation) (`KismetMathLibrary.BreakTransform` (`SceneComponent.K2_GetComponentToWorld` (`self.PickableMagnet`))))
  (if (`PickableMagnetComponent.IsAvailable` (`self.PickableMagnet`))
    (for _array_element (`self.LinkedPedestral`)
      (bind _currentpickable (`PickableMagnetComponent.CurrentPickable` (`/Game/TechnicalTest/Blueprints/Pedestral_BP.PickableMagnet` _array_element)))
      ;[1 1 1] Are all pedestral occupied
      (bind _output_get (set `local.bValid` (and (`KismetSystemLibrary.IsValid` _currentpickable) (`local.bValid`))))
      (if _output_get
        (`KismetArrayLibrary.Array_Add` (`local.Elements`) (`self.GetComponentByClass` (`ActorComponent.GetOwner` _currentpickable) "/Script/TechnicalTest.ElementalComponent"))))
    (if (`local.bValid`)
      (bind _returnvalue (`ElementalComponent.MergeElement` (`local.Elements`)))
      (bind _output (`|GetArrayItem` _returnvalue))
      ;[1 1 1] is this particuliar merge is valid for this shrine
      (if (or (`KismetArrayLibrary.Array_Contains` _splitormergevalidstate _output) (== (`KismetArrayLibrary.Array_Length` _splitormergevalidstate) 0))
        (bind _returnvalue_2 (`|SpawnActorFromClass` "/Game/TechnicalTest/Blueprints/ElementalSphere_BP.ElementalSphere_BP_C" (`KismetMathLibrary.MakeTransform` _returnvalue_location _returnvalue_rotation) "AlwaysSpawn" "OverrideRootScale" null null))
        (`/Game/TechnicalTest/Blueprints/ElementalSphere_BP.SetElement` _returnvalue_2 _output)
        (`PickableMagnetComponent.AttachPickable` (`self.PickableMagnet`) (`self.GetComponentByClass` _returnvalue_2 "/Script/TechnicalTest.PickableComponent"))
        (for (_array_element_2 _array_index) (`self.LinkedPedestral`)
          (bind _output_2 (`|GetArrayItem` _returnvalue (+ _array_index 1)))
          ;[1 1 1] Shall I destroy the merge or change its elemental type
          (if (== _output_2 0)
            (`/Game/TechnicalTest/Blueprints/Pedestral_BP.DestroyElementalSphere` _array_element_2)
            (else
              (`/Game/TechnicalTest/Blueprints/Pedestral_BP.SetElementalSphereElement` _array_element_2 _output_2))))))))

(fn `UserConstructionScript`
  (`SceneComponent.SetVisibility` (`self.PlusSignMesh`) false false)
  (`SceneComponent.SetVisibility` (`self.EqualSignMesh`) false false)
  (`SceneComponent.SetVisibility` (`self.EqualSignMesh1`) false false)
  (`SceneComponent.SetVisibility` (`self.MinusSignMesh`) false false)
  (`SceneComponent.SetVisibility` (`self.SplitSignMesh3`) false false)
  (`SceneComponent.SetVisibility` (`self.MergeSignMesh1`) false false)
  (`SceneComponent.SetVisibility` (`self.SplitSignMesh4`) false false)
  (`SceneComponent.SetVisibility` (`self.MergeSignMesh2`) false false)
  (`SceneComponent.SetVisibility` (`self.MergeSignMesh3`) false false)
  (`SceneComponent.SetVisibility` (`self.MergeSignMesh4`) false false)
  (`SceneComponent.SetVisibility` (`self.MergeSignMesh5`) false false)
  (`SceneComponent.SetVisibility` (`self.SplitSignMesh2`) false false)
  (`SceneComponent.SetVisibility` (`self.SplitSignMesh5`) false false)
  (`SceneComponent.SetVisibility` (`self.Base`) false false)
  (switch `/Game/TechnicalTest/Enum/ElementImbueType` (`self.ImbueType`)
    (:`NewEnumerator0`
      (`SceneComponent.SetVisibility` (`self.EqualSignMesh1`) true false)
      (`SceneComponent.SetVisibility` (`self.EqualSignMesh`) true false)
      (`SceneComponent.SetVisibility` (`self.Base`) true false))
    (:`NewEnumerator1`
      (`SceneComponent.SetVisibility` (`self.MinusSignMesh`) true false)
      (`SceneComponent.SetVisibility` (`self.PlusSignMesh`) true false)
      (`SceneComponent.SetVisibility` (`self.Base`) true false))
    (:`NewEnumerator2`
      (`SceneComponent.SetVisibility` (`self.MinusSignMesh`) true false)
      (`SceneComponent.SetVisibility` (`self.Base`) true false))
    (:`NewEnumerator3`
      (`SceneComponent.SetVisibility` (`self.MinusSignMesh`) true false)
      (`SceneComponent.SetVisibility` (`self.SplitSignMesh1`) true false)
      (`SceneComponent.SetVisibility` (`self.SplitSignMesh2`) true false)
      (`SceneComponent.SetVisibility` (`self.SplitSignMesh3`) true false)
      (`SceneComponent.SetVisibility` (`self.SplitSignMesh4`) true false)
      (`SceneComponent.SetVisibility` (`self.SplitSignMesh5`) true false))
    (:`NewEnumerator4`
      (`SceneComponent.SetVisibility` (`self.MergeSignMesh1`) true false)
      (`SceneComponent.SetVisibility` (`self.MergeSignMesh2`) true false)
      (`SceneComponent.SetVisibility` (`self.MergeSignMesh3`) true false)
      (`SceneComponent.SetVisibility` (`self.MergeSignMesh4`) true false)
      (`SceneComponent.SetVisibility` (`self.MergeSignMesh5`) true false))))